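; Base game mode for a tank game that tracks joining players and spawns their chosen tank.
; OnPostLogin adds each new player controller to the AllPCs list.
; SpawnPlayer destroys the controller's current pawn, spawns one of the MK-2 to MK-7 tank Blueprints by selection, and possesses it.
; Each spawn uses a transform from a PlayerStart picked at random among all those in the level.
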(event `Event OnPostLogin`
  (params (NewPlayer :type "PlayerController Object Reference"))
  (`KismetArrayLibrary.Array_Add` (`self.All_PCs`) NewPlayer))

(fn `Find_Random_PlayerStart`
  (returns (PlayerStart_Transform :type "Transform Structure (by ref)"))
  (bind _outactors (`GameplayStatics.GetAllActorsOfClass` "/Script/Engine.PlayerStart"))
  (return (`self.GetTransform` (`|GetArrayItem` _outactors (`KismetMathLibrary.RandomIntegerInRange` 0 (- (`KismetArrayLibrary.Array_Length` _outactors) 1))))))

(fn `Spawn_Player`
  (params (Player_Controller :type "PlayerController Object Reference") (TankChoosen :type String))
  (locals (PlayerController :type "PlayerController Object Reference"))
  (bind _returnvalue (`Controller.K2_GetPawn` Player_Controller))
  (set `local.PlayerController` Player_Controller)
  (`/Engine/EditorBlueprintResources/StandardMacros.IsValid` _returnvalue
    (:`Is Valid`
      (`self.K2_DestroyActor` _returnvalue))
    (:`Is Not Valid`
      _))
  (switch `string` TankChoosen
    (:`MK-2`
      (bind _returnvalue_2 (`|SpawnActorFromClass` "/Game/Blueprints/BP_MK2.BP_MK2_C" (`self.Find_Random_PlayerStart`) "Undefined" "MultiplyWithRoot" null null))
      (`Controller.Possess` (`local.PlayerController`) _returnvalue_2))
    (:`MK-3`
      (bind _returnvalue_3 (`|SpawnActorFromClass` "/Game/Blueprints/BP_MK3.BP_MK3_C" (`self.Find_Random_PlayerStart`) "Undefined" "MultiplyWithRoot" null null))
      (`Controller.Possess` (`local.PlayerController`) _returnvalue_3))
    (:`MK-4`
      (bind _returnvalue_4 (`|SpawnActorFromClass` "/Game/Blueprints/BP_MK4.BP_MK4_C" (`self.Find_Random_PlayerStart`) "Undefined" "MultiplyWithRoot" null null))
      (`Controller.Possess` (`local.PlayerController`) _returnvalue_4))
    (:`MK-5`
      (bind _returnvalue_5 (`|SpawnActorFromClass` "/Game/Blueprints/BP_MK5.BP_MK5_C" (`self.Find_Random_PlayerStart`) "Undefined" "MultiplyWithRoot" null null))
      (`Controller.Possess` (`local.PlayerController`) _returnvalue_5))
    (:`MK-6`
      (bind _returnvalue_6 (`|SpawnActorFromClass` "/Game/Blueprints/BP_MK6.BP_MK6_C" (`self.Find_Random_PlayerStart`) "Undefined" "MultiplyWithRoot" null null))
      (`Controller.Possess` (`local.PlayerController`) _returnvalue_6))
    (:`MK-7`
      (bind _returnvalue_7 (`|SpawnActorFromClass` "/Game/Blueprints/BP_MK7.BP_MK7_C" (`self.Find_Random_PlayerStart`) "Undefined" "MultiplyWithRoot" null null))
      (`Controller.Possess` (`local.PlayerController`) _returnvalue_7))))

(fn `UserConstructionScript`)