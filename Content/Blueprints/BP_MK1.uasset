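; BP_MK1 is a player-controlled hover ship with an aimable turret and cannon, driven by Enhanced Input.
; Each tick, Fly lowers the body's center of mass and tilts Reactor-tagged hover thrusters' parents in yaw-compensated world space, oppositely front and rear for rotation.
; ControlTurret rotates a pitch-clamped spring arm, copies it to a target, then interpolates turret yaw and cannon pitch toward it.
; Both functions flip controls when the hull rolls upside down.
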(event `self.ReceiveBeginPlay`
  (`GameplayStatics.SetGlobalTimeDilation` 1.0)
  (`|ExecutionSequence`
    (:`then_0`
      ; Inputs
      (bind _asplayer_controller (cast `PlayerController` (`self.GetController`)))
      (`EnhancedInputSubsystemInterface.AddMappingContext` (pcsubsystem `EnhancedInputLocalPlayerSubsystem` _asplayer_controller) "/Game/Inputs/IMC_Ship.IMC_Ship" 0 (struct)))
    (:`then_1`
      ; Set thruster
      (for _array_element (`self.GetComponentsByTag` "/Game/Blueprints/BP_HoverComponent.BP_HoverComponent_C" "Reactor")
        (`SceneComponent.K2_SetWorldLocation` _array_element (`SceneComponent.K2_GetComponentLocation` (`|GetArrayItem` (`SceneComponent.GetParentComponents` _array_element))) false false)))))

(event `self.ReceiveTick`
  (params (DeltaSeconds :type "Float (single-precision)"))
  (`self.Fly` (`self.Body`) (`|GetInputActionValue`) (`|GetInputActionValue`))
  (`self.Control Turret` (`|GetInputActionValue`) (`|GetInputActionValue`) (`self.Turret`) (`self.Cannon`) (`self.TurretTarget`) (`self.SpringArm`)))

(fn `Control Turret`
  (params (Rotation :type "Float (double-precision)") (Elevation :type "Float (double-precision)") (Turret :type "StaticMeshComponent Object Reference") (Gun :type "StaticMeshComponent Object Reference") (TargetTurret :type "StaticMeshComponent Object Reference") (CameraArm :type "SpringArmComponent Object Reference"))
  (bind _rotation (`local.Rotation`))
  (bind _elevation (`local.Elevation`))
  (bind _cameraarm (`local.CameraArm`))
  (bind _cameraarm_2 (`local.CameraArm`))
  (bind (_relativerotation_roll _relativerotation_pitch _relativerotation_yaw) (`KismetMathLibrary.BreakRotator` (`SceneComponent.RelativeRotation` _cameraarm_2)))
  (bind (_relativerotation_roll_2 _relativerotation_pitch_2 _relativerotation_yaw_2) (`KismetMathLibrary.BreakRotator` (`SceneComponent.RelativeRotation` (`local.TargetTurret`))))
  (bind (_relativerotation_roll_3 _relativerotation_pitch_3 _relativerotation_yaw_3) (`KismetMathLibrary.BreakRotator` (`SceneComponent.RelativeRotation` (`local.Turret`))))
  (bind (_returnvalue_roll _returnvalue_pitch _returnvalue_yaw) (`KismetMathLibrary.BreakRotator` (`KismetMathLibrary.RInterpTo` (`KismetMathLibrary.MakeRotator` _relativerotation_roll_3 _relativerotation_pitch_3 _relativerotation_yaw_3) (`KismetMathLibrary.MakeRotator` _relativerotation_roll_2 (+ _relativerotation_pitch_2 (* 10.0 (`self.Returned Coef`))) _relativerotation_yaw_2) (`GameplayStatics.GetWorldDeltaSeconds`) 3.0)))
  (`|ExecutionSequence`
    (:`then_0`
      (if (`self.isReturned`)
        (`SceneComponent.K2_AddRelativeRotation` _cameraarm_2 (`KismetMathLibrary.MakeRotator` 0.0 _elevation (* _rotation -1.0)) false false)
        (else
          (`SceneComponent.K2_AddRelativeRotation` _cameraarm_2 (`KismetMathLibrary.MakeRotator` 0.0 _elevation _rotation) false false)))
      (`SceneComponent.K2_SetRelativeRotation` _cameraarm (`KismetMathLibrary.MakeRotator` _relativerotation_roll (`KismetMathLibrary.FClamp` _relativerotation_pitch -40.0 30.0) _relativerotation_yaw) false false)
      (`SceneComponent.K2_SetRelativeRotation` (`local.TargetTurret`) (`SceneComponent.RelativeRotation` _cameraarm) false false))
    (:`then_1`
      (if (`self.isReturned`)
        (set `self.Returned Coef` -1.0)
        (else
          (set `self.Returned Coef` 1.0))))
    (:`then_2`
      (`SceneComponent.K2_SetRelativeRotation` (`local.Turret`) (`KismetMathLibrary.MakeRotator` 0.0 0.0 _returnvalue_yaw) false false)
      (`SceneComponent.K2_SetRelativeRotation` (`local.Gun`) (`KismetMathLibrary.MakeRotator` 0.0 (* _returnvalue_pitch 20.0)) false false))))

(fn `Fly`
  (params (Body :type "StaticMeshComponent Object Reference") (Movement :type "Vector2D Structure") (Rotation :type "Float (double-precision)"))
  (bind (_returnvalue_roll _returnvalue_pitch _returnvalue_yaw) (`KismetMathLibrary.BreakRotator` (`SceneComponent.K2_GetComponentRotation` (`self.Main Part`))))
  (bind (_returnvalue_roll_2 _returnvalue_pitch_2 _returnvalue_yaw_2) (`KismetMathLibrary.BreakRotator` (`SceneComponent.K2_GetComponentRotation` (`self.Main Part`))))
  (bind _returnvalue_roll_3 (`KismetMathLibrary.BreakRotator` (`SceneComponent.K2_GetComponentRotation` (`self.Main Part`))))
  (bind _returnvalue (`KismetMathLibrary.DegCos` _returnvalue_yaw))
  (bind _returnvalue_2 (`KismetMathLibrary.DegSin` _returnvalue_yaw))
  (bind _returnvalue_3 (`KismetMathLibrary.DegCos` _returnvalue_yaw_2))
  (bind _returnvalue_4 (`KismetMathLibrary.DegSin` _returnvalue_yaw_2))
  (bind (_returnvalue_roll_4 _returnvalue_pitch_3) (`KismetMathLibrary.BreakRotator` (`KismetMathLibrary.MakeRotator` (* (`self.Sides`) (`self.Angle`) -1.0) (+ (* (`self.Front`) (`self.Angle`) -1.0) (* (`self.Rotate`) 15.0)))))
  (bind (_returnvalue_roll_5 _returnvalue_pitch_4) (`KismetMathLibrary.BreakRotator` (`KismetMathLibrary.MakeRotator` (* (`self.Sides`) (`self.Angle`) -1.0) (+ (* (`self.Front`) (`self.Angle`) -1.0) (* (`self.Rotate`) -15.0)))))
  ; Manage Inverted/Not behavior
  (set `self.Main Part` Body)
  (bind _output_get (set `self.isReturned` (or (< _returnvalue_roll_3 -90.0) (> _returnvalue_roll_3 90.0))))
  (if _output_get
    (set `self.Rotate` (* Rotation -1.0))
    (else
      (set `self.Rotate` Rotation)))
  (set `self.Front` Movement_Y)
  (set `self.Sides` Movement_X)
  (bind _asprimitive_component (cast `PrimitiveComponent` (`self.Main Part`)))
  ; Manage center of mass
  (`PrimitiveComponent.SetCenterOfMass` _asprimitive_component (0.0 0.0 -100.0) "None")
  (for _array_element (`self.GetComponentsByTag` "/Game/Blueprints/BP_HoverComponent.BP_HoverComponent_C" "Reactor")
    (bind _componenttags (`ActorComponent.ComponentTags` _array_element))
    (if (`KismetArrayLibrary.Array_Contains` _componenttags "Right")
      (bind _output (`|GetArrayItem` (`SceneComponent.GetParentComponents` _array_element)))
      ; Rear Thrusters
      (`SceneComponent.K2_SetWorldRotation` _output (`KismetMathLibrary.MakeRotator` (- (* _returnvalue _returnvalue_roll_4) (* _returnvalue_2 _returnvalue_pitch_3)) (+ (* _returnvalue_roll_4 _returnvalue_2) (* _returnvalue _returnvalue_pitch_3)) -1.0) false false)
      (elif (`KismetArrayLibrary.Array_Contains` _componenttags "Left")
        ; Front Thrusters
        (`SceneComponent.K2_SetWorldRotation` _output (`KismetMathLibrary.MakeRotator` (- (* _returnvalue_3 _returnvalue_roll_5) (* _returnvalue_4 _returnvalue_pitch_4)) (+ (* _returnvalue_roll_5 _returnvalue_4) (* _returnvalue_3 _returnvalue_pitch_4)) -1.0) false false)))))

(fn `UserConstructionScript`)