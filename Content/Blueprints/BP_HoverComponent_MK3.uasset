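; BP_HoverComponent_MK3 is a scene component that applies a hover force at its location to the owner's physics root.
; Each tick it sphere-traces straight down over Height and shows its first child component only on a hit.
; On a hit, a spring-damper turns compression and its rate of change into force along the attach parent's up vector.
; The stiffness term scales with the body's mass, while the damping term does not.
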(event `self.ReceiveBeginPlay`
  (bind _asprimitive_component (cast `PrimitiveComponent` (`Actor.RootComponent` (`self.GetOwner`))))
  (set `self.Owner` _asprimitive_component))

(event `self.ReceiveTick`
  (params (DeltaSeconds :type "Float (single-precision)"))
  (bind _returnvalue (`self.K2_GetComponentLocation`))
  (bind _height (`self.Height`))
  (bind (_outhit _returnvalue_2) (`KismetSystemLibrary.SphereTraceSingle` _returnvalue (- _returnvalue (* (`self.Height`) (0.0 0.0 1.0))) 20.0 "TraceTypeQuery1" false (`|MakeArray` (`self.GetOwner`))))
  (`self.SetVisibility` (`self.GetChildComponent` 0) _returnvalue_2 false)
  (if _returnvalue_2
    (bind _returnvalue_3 (/ (- _height (`.Distance` (`GameplayStatics.BreakHitResult` _outhit))) _height))
    (set `self.Hover Force` (+ (* (/ (- _returnvalue_3 (`self.Previous Compression`)) (`GameplayStatics.GetWorldDeltaSeconds`)) (`self.Damping`)) (* _returnvalue_3 (`self.Stiffness`) (`PrimitiveComponent.GetMass` (`self.Owner`)))))
    (set `self.Previous Compression` _returnvalue_3)
    (`PrimitiveComponent.AddForceAtLocation` (`self.Owner`) (* (`KismetMathLibrary.GetUpVector` (`self.K2_GetComponentRotation` (`self.GetAttachParent`))) (`self.Hover Force`)) _returnvalue "None")))