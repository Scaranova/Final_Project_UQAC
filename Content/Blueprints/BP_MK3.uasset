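; Player-controlled MK3 hover tank with a turret cannon, scope view, health and destruction effects.
; Local Tick input, firing and damage pass through ROS-to-MC event pairs; the shield ability only sets a cooldown.
; Fly tilts tagged hover thrusters to steer, shifting center of mass and inverting rotation when flipped.
; ControlTurret eases turret and gun toward the camera arm with rate-limited yaw, while Fire spawns BP_AP100 with physical recoil.
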(event `self.ReceiveBeginPlay`
  (`ActorComponent.SetActive` (`self.Scope`) false false)
  (`|ExecutionSequence`
    (:`then_0`
      (`KismetSystemLibrary.Delay` 0.1)
      ; Inputs
      (bind _asplayer_controller (cast `PlayerController` (`self.GetController`)))
      (`EnhancedInputSubsystemInterface.AddMappingContext` (pcsubsystem `EnhancedInputLocalPlayerSubsystem` _asplayer_controller) "/Game/Inputs/IMC_Ship.IMC_Ship" 0 (struct)))
    (:`then_1`
      (for _array_element (`self.GetComponentsByTag` "/Game/Blueprints/BP_HoverComponent_MK3.BP_HoverComponent_MK3_C" "Reactor")
        (`SceneComponent.K2_SetWorldLocation` _array_element (`SceneComponent.K2_GetComponentLocation` (`|GetArrayItem` (`SceneComponent.GetParentComponents` _array_element))) false false)))))

(event `self.ReceiveTick`
  (params (DeltaSeconds :type "Float (single-precision)"))
  (bind _cooldown (`self.Cooldown`))
  (bind _ability_cooldonw (`self.Ability_Cooldonw`))
  (if (`self.IsLocallyControlled`)
    (if (> _ability_cooldonw 0.0)
      (set `self.Ability_Cooldonw` (- _ability_cooldonw DeltaSeconds)))
    (if (> _cooldown 0.0)
      (set `self.Cooldown` (- _cooldown DeltaSeconds)))
    (`self.ROS_Fly_ControlTurret3` (`self.Base`) (`|GetInputActionValue`) (`|GetInputActionValue`) (`|GetInputActionValue`) (`|GetInputActionValue`) (`self.Turret`) (`self.Gun_Mount`) (`self.Turret_Target`) (`self.SpringArm`))))

(event `ROS_Fly_ControlTurret3`
  (params (Body :type "StaticMeshComponent Object Reference") (Movement :type "Vector2D Structure") (Rotation :type "Float (double-precision)") (Rotation2 :type "Float (double-precision)") (Elevation :type "Float (double-precision)") (Turret :type "StaticMeshComponent Object Reference") (Gun :type "StaticMeshComponent Object Reference") (TargetTurret :type "StaticMeshComponent Object Reference") (CameraArm :type "SpringArmComponent Object Reference"))
  (`self.MC_Fly_ControlTurret3` Body Movement Rotation Rotation2 Elevation Turret Gun TargetTurret CameraArm))

(event `MC_Fly_ControlTurret3`
  (params (Body :type "StaticMeshComponent Object Reference") (Movement :type "Vector2D Structure") (Rotation :type "Float (double-precision)") (Rotation2 :type "Float (double-precision)") (Elevation :type "Float (double-precision)") (Turret :type "StaticMeshComponent Object Reference") (Gun :type "StaticMeshComponent Object Reference") (TargetTurret :type "StaticMeshComponent Object Reference") (CameraArm :type "SpringArmComponent Object Reference"))
  (`self.Fly` Body Movement Rotation)
  (`self.Control Turret` Rotation2 Elevation Turret Gun TargetTurret CameraArm))

(event `EnhancedInput|/Game/Inputs/Actions/IA_Fire`
  (params (ActionValue :type Boolean) (ElapsedSeconds :type "Float (double-precision)") (TriggeredSeconds :type "Float (double-precision)") (InputAction :type "InputAction Object Reference" :default "/Game/Inputs/Actions/IA_Fire.IA_Fire"))
  (:`Started`
    (if (<= (`self.Cooldown`) 0.0)
      (`self.ROS_Fire3`))))

(event `ROS_Fire3`
  (`self.MC_Fire3`))

(event `MC_Fire3`
  (if (not (`self.Destroyed`))
    (bind _barrel (`self.Fire` (`self.Cannon`) (`self.Base`) 2.5))
    (set `self.Barrel loc` (`SceneComponent.RelativeLocation` _barrel))
    (bind (_direction _gun_track_recoil) (`Timeline|Gun_Recoil` :!via `PlayFromStart`)
      (:`Update`
        (`SceneComponent.K2_SetRelativeLocation` _barrel (+ (`self.Barrel loc`) (* _gun_track_recoil (7.0 0.0 0.0))) false false)))))

(event `EnhancedInput|/Game/Inputs/Actions/IA_decouple_camera`
  (params (ActionValue :type Boolean) (ElapsedSeconds :type "Float (double-precision)") (TriggeredSeconds :type "Float (double-precision)") (InputAction :type "InputAction Object Reference" :default "/Game/Inputs/Actions/IA_decouple_camera.IA_decouple_camera"))
  (:`Started`
    (set `self.Camera_lock` false))
  (:`Completed`
    (set `self.Camera_lock` true)))

(event `EnhancedInput|/Game/Inputs/Actions/IA_Scope`
  (params (ActionValue :type Boolean) (ElapsedSeconds :type "Float (double-precision)") (TriggeredSeconds :type "Float (double-precision)") (InputAction :type "InputAction Object Reference" :default "/Game/Inputs/Actions/IA_Scope.IA_Scope"))
  (bind _destroyed (`self.Destroyed`))
  (:`Started`
    (if (not _destroyed)
      (`ActorComponent.SetActive` (`self.Scope`) true false)
      (`ActorComponent.SetActive` (`self.Camera`) false false)
      (bind _returnvalue (`|CreateWidget` "/Game/Aiming_UI/WB_Aiim_cursor.WB_Aiim_cursor_C"))
      (bind _output_get (set `self.Aim` _returnvalue))
      (`UserWidget.AddToViewport` _output_get 0)))
  (:`Completed`
    (if (not _destroyed)
      (`ActorComponent.SetActive` (`self.Scope`) false false)
      (`ActorComponent.SetActive` (`self.Camera`) true false)
      (`Widget.RemoveFromParent` (`self.Aim`)))))

(event `ROS_TakeDamage3`
  (params (Damage :type "Float (double-precision)"))
  (`self.MC_TakeDamage3` Damage))

(event `/Game/Blueprints/BP_Tanks.Take Damage`
  (params (Damage :type "Float (double-precision)"))
  (`self.ROS_TakeDamage3` Damage))

(event `MC_TakeDamage3`
  (params (Damage :type "Float (double-precision)"))
  (bind _output_get (set `self.HP` (- (`self.HP`) Damage)))
  (if (and (<= _output_get 0.0) (not (`self.Destroyed`)))
    (for _array_element (`self.K2_GetComponentsByClass` "/Game/Blueprints/BP_HoverComponent_MK3.BP_HoverComponent_MK3_C")
      (`ActorComponent.SetActive` (`SceneComponent.GetChildComponent` _array_element 0) false false)
      (set `/Game/Blueprints/BP_HoverComponent_MK3.Height` 0.0 _array_element)
      (for _array_element_2 (`self.K2_GetComponentsByClass` "/Script/Engine.StaticMeshComponent")
        (for (_ _array_index) (`MeshComponent.GetMaterials` _array_element_2)
          (`PrimitiveComponent.SetMaterial` _array_element_2 _array_index "/Game/Assets/3D_models/MK4/Material_008.Material_008"))))
    (`NiagaraFunctionLibrary.SpawnSystemAtLocation` "/Game/Assets/Particles/NS_Impact_Destruction.NS_Impact_Destruction" (`self.K2_GetActorLocation`) (struct) (2.0 2.0 2.0))
    (bind _returnvalue (`NiagaraFunctionLibrary.SpawnSystemAttached` "/Game/Assets/Particles/NS_Fire_Post_Destruction.NS_Fire_Post_Destruction" (`self.RootComponent`) "None" (0.0 0.0 0.0) (struct) "KeepRelativeOffset"))
    (`SceneComponent.SetWorldScale3D` _returnvalue (1.0 1.0 1.0))
    (set `self.Destroyed` true)))

(event `/Game/Blueprints/BP_Tanks.Heal`
  (params (Quantity :type "Float (double-precision)"))
  (bind _hp (`self.HP`))
  (if (< _hp (`self.Max_HP`))
    (set `self.HP` (+ Quantity _hp))))

(event `EnhancedInput|/Game/Inputs/Actions/IA_Ability`
  (params (ActionValue :type Boolean) (ElapsedSeconds :type "Float (double-precision)") (TriggeredSeconds :type "Float (double-precision)") (InputAction :type "InputAction Object Reference" :default "/Game/Inputs/Actions/IA_Ability.IA_Ability"))
  (:`Started`
    (`self.Ability_Shield`)))

(event `self.Turret_collision.OnComponentBeginOverlap`
  (params (OverlappedComponent :type "PrimitiveComponent Object Reference") (OtherActor :type "Actor Object Reference") (OtherComp :type "PrimitiveComponent Object Reference") (OtherBodyIndex :type Integer) (bFromSweep :type Boolean) (SweepResult :type "HitResult Structure (by ref)"))
  (if (!= (`self.GetOwner` OtherActor) null)
    (message `/Game/Blueprints/SHell/BP_Shell.Impact` OtherActor self)))

(event `self.Base_collision.OnComponentBeginOverlap`
  (params (OverlappedComponent :type "PrimitiveComponent Object Reference") (OtherActor :type "Actor Object Reference") (OtherComp :type "PrimitiveComponent Object Reference") (OtherBodyIndex :type Integer) (bFromSweep :type Boolean) (SweepResult :type "HitResult Structure (by ref)"))
  (if (!= (`self.GetOwner` OtherActor) null)
    (message `/Game/Blueprints/SHell/BP_Shell.Impact` OtherActor self)))

(event `ROS_Fire`)

(event `ROS_Fly_ControlTurret`
  (params (Body :type "StaticMeshComponent Object Reference") (Movement :type "Vector2D Structure") (Rotation :type "Float (double-precision)") (Rotation2 :type "Float (double-precision)") (Elevation :type "Float (double-precision)") (Turret :type "StaticMeshComponent Object Reference") (Gun :type "StaticMeshComponent Object Reference") (TargetTurret :type "StaticMeshComponent Object Reference") (CameraArm :type "SpringArmComponent Object Reference")))

(event `ROS_TakeDamage`
  (params (Damage :type "Float (double-precision)")))

(fn `Ability_Shield`
  (if (<= (`self.Ability_Cooldonw`) 0.0)
    (set `self.Ability_Cooldonw` 5.0)))

(fn `Control Turret`
  (params (Rotation :type "Float (double-precision)") (Elevation :type "Float (double-precision)") (Turret :type "StaticMeshComponent Object Reference") (Gun :type "StaticMeshComponent Object Reference") (TargetTurret :type "StaticMeshComponent Object Reference") (CameraArm :type "SpringArmComponent Object Reference"))
  (bind _targetturret (`local.TargetTurret`))
  (bind _rotation (`local.Rotation`))
  (bind _elevation (`local.Elevation`))
  (bind _cameraarm (`local.CameraArm`))
  (bind _cameraarm_2 (`local.CameraArm`))
  (bind _turret (`local.Turret`))
  (bind (_returnvalue_roll _returnvalue_pitch _returnvalue_yaw) (`KismetMathLibrary.BreakRotator` (`SceneComponent.K2_GetComponentRotation` _cameraarm)))
  (bind (_returnvalue_roll_2 _returnvalue_pitch_2 _returnvalue_yaw_2) (`KismetMathLibrary.BreakRotator` (`SceneComponent.K2_GetComponentRotation` (`self.RootComponent`))))
  (bind (_relativerotation_roll _relativerotation_pitch) (`KismetMathLibrary.BreakRotator` (`SceneComponent.RelativeRotation` (`local.Gun`))))
  (bind (_relativerotation_roll_2 _relativerotation_pitch_2 _relativerotation_yaw) (`KismetMathLibrary.BreakRotator` (`SceneComponent.RelativeRotation` _cameraarm_2)))
  (bind (_relativerotation_roll_3 _relativerotation_pitch_3) (`KismetMathLibrary.BreakRotator` (`SceneComponent.RelativeRotation` _cameraarm)))
  (bind (_relativerotation_roll_4 _relativerotation_pitch_4 _relativerotation_yaw_2) (`KismetMathLibrary.BreakRotator` (`SceneComponent.RelativeRotation` _targetturret)))
  (bind (_relativerotation_roll_5 _relativerotation_pitch_5 _relativerotation_yaw_3) (`KismetMathLibrary.BreakRotator` (`SceneComponent.RelativeRotation` (`local.TargetTurret`))))
  (bind (_relativerotation_roll_6 _relativerotation_pitch_6 _relativerotation_yaw_4) (`KismetMathLibrary.BreakRotator` (`SceneComponent.RelativeRotation` _turret)))
  (bind (_relativerotation_roll_7 _relativerotation_pitch_7 _relativerotation_yaw_5) (`KismetMathLibrary.BreakRotator` (`SceneComponent.RelativeRotation` (`local.Turret`))))
  (bind _returnvalue (`KismetMathLibrary.DegreesToRadians` _returnvalue_yaw_2))
  (bind (_returnvalue_roll_3 _returnvalue_pitch_3 _returnvalue_yaw_3) (`KismetMathLibrary.BreakRotator` (`KismetMathLibrary.RInterpTo` (`KismetMathLibrary.MakeRotator` _relativerotation_roll_7 _relativerotation_pitch _relativerotation_yaw_5) (`KismetMathLibrary.MakeRotator` _relativerotation_roll_5 (+ _relativerotation_pitch_5 (* 10.0 (`self.Returned Coef`))) _relativerotation_yaw_3) (`GameplayStatics.GetWorldDeltaSeconds`) 1.0)))
  (bind _returnvalue_2 (`KismetMathLibrary.DegCos` _returnvalue))
  (bind _returnvalue_3 (`KismetMathLibrary.DegSin` _returnvalue))
  (bind _returnvalue_4 (- _returnvalue_yaw_3 _relativerotation_yaw_4))
  (`|ExecutionSequence`
    (:`then_0`
      (if (`self.isReturned`)
        (`SceneComponent.K2_AddRelativeRotation` _cameraarm_2 (`KismetMathLibrary.MakeRotator` 0.0 _elevation (* _rotation -1.0)) false false)
        (else
          (`SceneComponent.K2_AddRelativeRotation` _cameraarm_2 (`KismetMathLibrary.MakeRotator` 0.0 _elevation _rotation) false false)))
      (`SceneComponent.K2_SetRelativeRotation` _cameraarm (`KismetMathLibrary.MakeRotator` _relativerotation_roll_2 (`KismetMathLibrary.FClamp` (`KismetMathLibrary.NormalizeAxis` _relativerotation_pitch_2) -40.0 30.0) _relativerotation_yaw) false false)
      (if (not (`self.Destroyed`))
        ; Limite la depression et l elevation du canon par rapport à celle calculée + ajustement de l elevation du canon
        (`SceneComponent.K2_SetWorldRotation` _targetturret (`KismetMathLibrary.MakeRotator` (- (* _returnvalue_roll_2 _returnvalue_2 0.0) (* _returnvalue_roll_2 _returnvalue_2 0.0)) (- (* _returnvalue_pitch_2 _returnvalue_3 _returnvalue_pitch) (* _returnvalue_pitch_2 _returnvalue_3 _returnvalue_pitch) (* _relativerotation_pitch_3 -1.0)) _returnvalue_yaw) false false)
        (`SceneComponent.K2_SetRelativeRotation` _targetturret (`KismetMathLibrary.MakeRotator` _relativerotation_roll_4 (`KismetMathLibrary.FClamp` (- _relativerotation_pitch_4 -2.0) -15.0 20.0) _relativerotation_yaw_2) false false)))
    (:`then_1`
      (if (`self.isReturned`)
        (set `self.Returned Coef` -1.0)
        (else
          (set `self.Returned Coef` 1.0))))
    (:`then_2`
      (if (`self.Camera_lock`)
        ; Limiter vitesse de rotation de la tourelle car sa vitesse dépendait de la distance a parcourir -> vitesse trop grande quand coup de souris
        (if (> (`KismetMathLibrary.Abs` _returnvalue_4) 355.0)
          (`SceneComponent.K2_AddRelativeRotation` _turret (`KismetMathLibrary.MakeRotator` 0.0 0.0 _returnvalue_4) false false)
          (else
            (`SceneComponent.K2_AddRelativeRotation` _turret (`KismetMathLibrary.MakeRotator` 0.0 0.0 (`KismetMathLibrary.FClamp` _returnvalue_4 -0.4 0.4)) false false)))
        (`SceneComponent.K2_SetRelativeRotation` (`local.Gun`) (`KismetMathLibrary.MakeRotator` 0.0 _returnvalue_pitch_3) false false)))))

(fn `Fire`
  (params (Cannon_Barrel :type "StaticMeshComponent Object Reference") (Body :type "StaticMeshComponent Object Reference") (Cooldown :type "Float (double-precision)"))
  (returns (Barrel :type "StaticMeshComponent Object Reference"))
  (bind _returnvalue (`SceneComponent.K2_GetComponentLocation` Cannon_Barrel))
  (bind _returnvalue_2 (`SceneComponent.K2_GetComponentRotation` Cannon_Barrel))
  (if (not (`self.Destroyed`))
    (`PrimitiveComponent.AddImpulseAtLocation` Body (* (`SceneComponent.GetForwardVector` Cannon_Barrel) 200000.0 -1.0) _returnvalue "None")
    (`NiagaraFunctionLibrary.SpawnSystemAtLocation` "/Game/Assets/Particles/NS_Fire_Smoke.NS_Fire_Smoke" _returnvalue _returnvalue_2 (3.0 3.0 3.0))
    (bind _returnvalue_3 (`|SpawnActorFromClass` "/Game/Blueprints/SHell/BP_AP-100.BP_AP-100_C" (`KismetMathLibrary.MakeTransform` (+ _returnvalue (0.0 0.0 0.0)) _returnvalue_2) "AdjustIfPossibleButAlwaysSpawn" "MultiplyWithRoot" null null))
    (`self.SetOwner` _returnvalue_3 self)
    (set `self.Cooldown` Cooldown)
    (return (`local.Cannon_Barrel`))))

(fn `Fly`
  (params (Body :type "StaticMeshComponent Object Reference") (Movement :type "Vector2D Structure") (Rotation :type "Float (double-precision)"))
  (bind _main_part (`self.Main Part`))
  (bind (_returnvalue_roll _returnvalue_pitch _returnvalue_yaw) (`KismetMathLibrary.BreakRotator` (`SceneComponent.K2_GetComponentRotation` (`self.Main Part`))))
  (bind (_returnvalue_roll_2 _returnvalue_pitch_2 _returnvalue_yaw_2) (`KismetMathLibrary.BreakRotator` (`SceneComponent.K2_GetComponentRotation` (`self.Main Part`))))
  (bind _returnvalue_roll_3 (`KismetMathLibrary.BreakRotator` (`SceneComponent.K2_GetComponentRotation` (`self.Main Part`))))
  (bind _returnvalue (`KismetMathLibrary.DegCos` _returnvalue_yaw))
  (bind _returnvalue_2 (`KismetMathLibrary.DegSin` _returnvalue_yaw))
  (bind _returnvalue_3 (`KismetMathLibrary.DegCos` _returnvalue_yaw_2))
  (bind _returnvalue_4 (`KismetMathLibrary.DegSin` _returnvalue_yaw_2))
  (bind (_returnvalue_roll_4 _returnvalue_pitch_3) (`KismetMathLibrary.BreakRotator` (`KismetMathLibrary.MakeRotator` (* (`self.Sides`) (`self.Angle`) -1.0) (+ (* (`self.Front`) (`self.Angle`) -1.0) (* (`self.Rotate`) 15.0)))))
  (bind (_returnvalue_roll_5 _returnvalue_pitch_4) (`KismetMathLibrary.BreakRotator` (`KismetMathLibrary.MakeRotator` (* (`self.Sides`) (`self.Angle`) -1.0) (+ (* (`self.Front`) (`self.Angle`) -1.0) (* (`self.Rotate`) -15.0)))))
  (if (not (`self.Destroyed`))
    ; Manage Inverted/Not behavior
    (set `self.Main Part` Body)
    (bind _output_get (set `self.isReturned` (or (< _returnvalue_roll_3 -90.0) (> _returnvalue_roll_3 90.0))))
    (if _output_get
      (set `self.Rotate` (`KismetMathLibrary.FInterpTo` (`self.Rotate`) (* Rotation -1.0) (`GameplayStatics.GetWorldDeltaSeconds`) 7.0))
      (bind _asprimitive_component (cast `PrimitiveComponent` _main_part))
      ; Manage center of mass
      (`PrimitiveComponent.SetCenterOfMass` _asprimitive_component (0.0 0.0 25.0) "None")
      (else
        (set `self.Rotate` (`KismetMathLibrary.FInterpTo` (`self.Rotate`) Rotation (`GameplayStatics.GetWorldDeltaSeconds`) 7.0))))
    (set `self.Front` (`KismetMathLibrary.FInterpTo` (`self.Front`) Movement_Y (`GameplayStatics.GetWorldDeltaSeconds`) 7.0))
    (set `self.Sides` (`KismetMathLibrary.FInterpTo` (`self.Sides`) Movement_X (`GameplayStatics.GetWorldDeltaSeconds`) 7.0))
    (bind _asprimitive_component_2 (cast `PrimitiveComponent` _main_part))
    (`PrimitiveComponent.SetCenterOfMass` _asprimitive_component_2 (0.0 0.0 -25.0) "None")
    (for _array_element (`self.GetComponentsByTag` "/Game/Blueprints/BP_HoverComponent_MK3.BP_HoverComponent_MK3_C" "Reactor")
      (bind _componenttags (`ActorComponent.ComponentTags` _array_element))
      (if (`KismetArrayLibrary.Array_Contains` _componenttags "Right")
        (bind _output (`|GetArrayItem` (`SceneComponent.GetParentComponents` _array_element)))
        ; Rear Thrusters
        (`SceneComponent.K2_SetWorldRotation` _output (`KismetMathLibrary.MakeRotator` (- (* _returnvalue _returnvalue_roll_4) (* _returnvalue_2 _returnvalue_pitch_3)) (+ (* _returnvalue_roll_4 _returnvalue_2) (* _returnvalue _returnvalue_pitch_3)) -1.0) false false)
        (elif (`KismetArrayLibrary.Array_Contains` _componenttags "Left")
          ; Front Thrusters
          (`SceneComponent.K2_SetWorldRotation` _output (`KismetMathLibrary.MakeRotator` (- (* _returnvalue_3 _returnvalue_roll_5) (* _returnvalue_4 _returnvalue_pitch_4)) (+ (* _returnvalue_roll_5 _returnvalue_4) (* _returnvalue_3 _returnvalue_pitch_4)) -1.0) false false))))))

(fn `MC_Fire`)

(fn `MC_Fly_ControlTurret`
  (params (Body1 :type "StaticMeshComponent Object Reference") (Movement1 :type "Vector2D Structure") (Rotation1 :type "Float (double-precision)") (Rotation21 :type "Float (double-precision)") (Elevation1 :type "Float (double-precision)") (Turret1 :type "StaticMeshComponent Object Reference") (Gun1 :type "StaticMeshComponent Object Reference") (TargetTurret1 :type "StaticMeshComponent Object Reference") (CameraArm1 :type "SpringArmComponent Object Reference")))

(fn `MC_TakeDamage`
  (params (Damage1 :type "Float (double-precision)")))

(fn `OnRep_Angle`)

(fn `OnRep_Front`)

(fn `OnRep_HoverDelta`)

(fn `OnRep_Previous HoverDelta`)

(fn `OnRep_Rotate`)

(fn `OnRep_Sides`)

(fn `UserConstructionScript`)