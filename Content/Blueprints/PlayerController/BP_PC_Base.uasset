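; Base player controller that requests the player's spawn with their chosen tank when play begins.
; BeginPlay sets game-only input, then the local controller reads the tank choice from BP_GameInstance and passes it to the SR_SpawnPlayer event.
; That event hands the controller and tank to GM_Base, which handles the spawn.
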(event `self.ReceiveBeginPlay`
  (`WidgetBlueprintLibrary.SetInputMode_GameOnly` self)
  (if (`self.IsLocalPlayerController`)
    (bind _asbp_game_instance (cast `/Game/Blueprints/GameInstance/BP_GameInstance` (`GameplayStatics.GetGameInstance`)))
    (`self.SR_SpawnPlayer` (`/Game/Blueprints/GameInstance/BP_GameInstance.TankChoosen` _asbp_game_instance))))

(event `SR_SpawnPlayer`
  (params (Tank :type String))
  (bind _asgm_base (cast `/Game/GM_Base` (`GameplayStatics.GetGameMode`)))
  (`/Game/GM_Base.Spawn_Player` _asgm_base self Tank))

(fn `UserConstructionScript`)