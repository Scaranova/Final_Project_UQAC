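; BP_AP-100 is a shell projectile, likely armor-piercing, that deals damage to a tank on impact and has a limited lifespan.
; Each tick it compares the Shell component's normalized velocity with the stored direction, treating a sharp change as an impact after the first frame.
; Impact spawns a Niagara effect, destroys the actor and sends Damage to the supplied tank, though the Tick-triggered call passes no tank.
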(event `self.ReceiveBeginPlay`
  (`self.SetLifeSpan` 10.0))

(event `self.ReceiveTick`
  (params (DeltaSeconds :type "Float (single-precision)"))
  (bind (_velocity_x _velocity_y _velocity_z) (`KismetMathLibrary.BreakVector` (`self.Velocity`)))
  (bind (_returnvalue_x _returnvalue_y _returnvalue_z) (`KismetMathLibrary.BreakVector` (`KismetMathLibrary.Normal` (`SceneComponent.GetComponentVelocity` (`self.Shell`)))))
  (if (and (not (`self.First frame`)) (> (`KismetMathLibrary.Abs` (`KismetMathLibrary.FMax` (- _returnvalue_x _velocity_x) (- _returnvalue_y _velocity_y) (- _returnvalue_z _velocity_z))) 0.3))
    (`/Game/Blueprints/SHell/BP_Shell.Impact` null)
    (else
      (set `self.Velocity` (`KismetMathLibrary.Normal` (`SceneComponent.GetComponentVelocity` (`self.Shell`))))
      (set `self.First frame` false))))

(event `/Game/Blueprints/SHell/BP_Shell.Impact`
  (params (`Tank Hitted` :type "Pawn Object Reference"))
  (`NiagaraFunctionLibrary.SpawnSystemAtLocation` "/Game/Assets/Particles/Shell/NS_Impact.NS_Impact" (`SceneComponent.K2_GetComponentLocation` (`self.Shell`)) (struct) (1.5 1.5 1.5))
  (`self.K2_DestroyActor`)
  (message `/Game/Blueprints/BP_Tanks.Take Damage` `Tank Hitted` (`self.Damage`)))

(fn `UserConstructionScript`)